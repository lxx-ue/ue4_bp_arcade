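; BP_Ball is a ball actor that moves in a straight line and bounces off whatever blocks it.
; Each Tick it sweeps a world offset from Direction, Speed and delta time, with no physics simulation calls.
; On a blocking hit it reflects Direction about the hit normal and cuts Speed by a tenth, clamped between Minlim and Maxlim.
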(event `self.ReceiveTick`
  (params (DeltaSeconds :type "Float (single-precision)"))
  (bind _sweephitresult (`self.K2_AddActorWorldOffset` (* (* (`self.direction`) (`self.speed`)) DeltaSeconds) true))
  (bind (_bblockinghit _binitialoverlap _time _distance _location _impactpoint _normal) (`GameplayStatics.BreakHitResult` _sweephitresult))
  (if _bblockinghit
    (set `self.direction` (`KismetMathLibrary.GetReflectionVector` (`self.direction`) _normal))
    (set `self.speed` (`KismetMathLibrary.FClamp` (* (`self.speed`) 0.9) (`self.minlim`) (`self.maxlim`)))))

(fn `UserConstructionScript`)