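; BP_Light is a blinking light actor that flashes its point light a set number of times when play begins.
; BeginPlay hides the light, then loops through a DoN node limited by Count, showing it for Duration and hiding it for a fixed pause.
; The construction script applies the Color variable to the light.
; Tick prints the actor's name and Count every frame as debug output.
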(event `self.ReceiveBeginPlay`
  (`SceneComponent.SetVisibility` (`self.PointLight`) false false)
  (`/Engine/EditorBlueprintResources/StandardMacros.Do N` (`self.count`) :!label _label
    (:`Exit`
      (`SceneComponent.SetVisibility` (`self.PointLight`) true false)
      (`KismetSystemLibrary.Delay` (`self.duration`))
      (`SceneComponent.SetVisibility` (`self.PointLight`) false false)
      (`KismetSystemLibrary.Delay` 0.5)
      (goto _label))))

(event `self.ReceiveTick`
  (params (DeltaSeconds :type "Float (single-precision)"))
  (`KismetSystemLibrary.PrintString` (`KismetStringLibrary.Concat_StrStr` (`KismetSystemLibrary.GetDisplayName` self) " " (`KismetStringLibrary.Conv_IntToString` (`self.count`))) true true (struct :`G` 0.66 :`B` 1.0 :`A` 1.0) DeltaSeconds))

(fn `UserConstructionScript`
  (`LightComponent.SetLightColor` (`self.PointLight`) (`self.color`) true))