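; BP_Block_green is a breakable block that loses health each time a BP_Ball hits it.
; Its Hit event ignores other actors, decrements Health and switches on the result.
; Depending on that value, the Cube mesh changes to an orange or black material to show damage, or the actor destroys itself at zero.
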(event `self.ReceiveHit`
  (params (MyComp :type "PrimitiveComponent Object Reference") (Other :type "Actor Object Reference") (OtherComp :type "PrimitiveComponent Object Reference") (bSelfMoved :type Boolean) (HitLocation :type "Vector Structure") (HitNormal :type "Vector Structure") (NormalImpulse :type "Vector Structure") (Hit :type "HitResult Structure (by ref)"))
  (cast `/Game/BP_Ball` Other)
  (bind _result (`/Engine/EditorBlueprintResources/StandardMacros.DecrementInt` (`self.health`))
    (:`  `
      (switch `int` _result
        (:`0`
          (`self.K2_DestroyActor`))
        (:`1`
          (`PrimitiveComponent.SetMaterial` (`self.Cube`) 0 "/Game/Materials/m_black1.m_black1"))
        (:`2`
          (`PrimitiveComponent.SetMaterial` (`self.Cube`) 0 "/Game/Materials/m_orange.m_orange"))))))

(fn `UserConstructionScript`
  (`parent.UserConstructionScript`))