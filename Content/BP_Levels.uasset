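; BP_Levels is the level manager that advances a block-clearing game through layouts stored in a Positions array.
; Every tick it counts BP_Block_simple actors and, when none remain, increments Level and starts the next level, guarded by a Stop flag.
; StartNextLevel destroys the current BP_Blocks, spawns a new one with that level's position string, and notifies the Pawn.
; ResetLevel rebuilds the current level.
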(event `self.ReceiveBeginPlay`
  (`self.StartNextLevel` (`self.level`)))

(event `self.ReceiveTick`
  (params (DeltaSeconds :type "Float (single-precision)"))
  (if (not (`self.stop`))
    (bind _outactors (`GameplayStatics.GetAllActorsOfClass` "/Game/Blocks/BP_Block_simple.BP_Block_simple_C"))
    (bind _output_get (set `self.to_next` (`KismetArrayLibrary.Array_Length` _outactors)))
    (if (== _output_get 0)
      (set `self.stop` true)
      (bind _result (`/Engine/EditorBlueprintResources/StandardMacros.IncrementInt` (`self.level`))
        (:`  `
          (`self.StartNextLevel` _result)
          (set `self.stop` false))))))

(fn `ResetLevel`
  (`self.StartNextLevel` (`self.level`)))

(fn `StartNextLevel`
  (params (level :type Integer))
  (bind _current_level (`self.current_level`)
    (:`then`
      (`/Game/BP_Blocks.Destroy` _current_level))
    (:`else`
      _))
  (bind _returnvalue (`|SpawnActorFromClass` "/Game/BP_Blocks.BP_Blocks_C" (`KismetMathLibrary.MakeTransform` (`self.start_pos`)) "Undefined" "OverrideRootScale" null (`|GetArrayItem` (`self.positions`) level) null))
  (set `self.current_level` _returnvalue)
  (`/Game/BP_Pawn.StartNewLevel` (`self.pawn`)))

(fn `UserConstructionScript`)