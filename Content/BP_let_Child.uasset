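; BP_let_Child is a child Blueprint actor whose Cube component shrinks when another actor overlaps it.
; Each begin-overlap event multiplies the Cube's current world scale by 0.95, so repeated overlaps compound the shrinking.
; The parent's overlap handler is not called, BeginPlay and Tick are disabled stubs, and the construction script only calls the parent.
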(event `self.ReceiveActorBeginOverlap`
  (params (OtherActor :type "Actor Object Reference"))
  (`SceneComponent.SetWorldScale3D` (`self.Cube`) (* (`SceneComponent.K2_GetComponentScale` (`self.Cube`)) 0.95)))

(fn `UserConstructionScript`
  (`parent.UserConstructionScript`))